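; BP_Note is an interactable note that opens a note reading UI when used.
; An overlap begin on the Widget component registers it as the combat character's interactable and reveals the prompt widget, while leaving the Trigger clears both.
; Tick turns the visible widget toward the player camera.
; UseInteractable hides the HUD, creates WBP_NoteUI, stores it on the controller and adds it to the viewport.
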(event OnComponentBeginOverlap(Widget)
  (params (OverlappedComponent :type Primitive%20Component%20Object%20Reference) (OtherActor :type Actor%20Object%20Reference) (OtherComp :type Primitive%20Component%20Object%20Reference) (OtherBodyIndex :type Integer) (bFromSweep :type Boolean) (SweepResult :type Hit%20Result%20Structure%20%28by%20ref%29))
  (bind _asbp_combat_character (Utilities|Casting|CastToBP_CombatCharacter OtherActor))
  (Variables|Default|SetPlayerRef _asbp_combat_character)
  (Default|SetInteractable (Variables|Default|GetPlayerRef) self)
  (Development|SetHiddeninGame (Variables|Default|GetWidget) false false))

(event OnComponentEndOverlap(Trigger)
  (params (OverlappedComponent :type Primitive%20Component%20Object%20Reference) (OtherActor :type Actor%20Object%20Reference) (OtherComp :type Primitive%20Component%20Object%20Reference) (OtherBodyIndex :type Integer))
  (bind _playerref (Variables|Default|GetPlayerRef))
  (if (== OtherActor _playerref)
    (Default|SetInteractable _playerref)
    (Development|SetHiddeninGame (Variables|Default|GetWidget) true false)))

(event EventBeginPlay
  (|CallParentFunction)
  (Development|SetHiddeninGame (Variables|Default|GetWidget) true false))

(event EventTick
  (params (DeltaSeconds :type Float%20%28single-precision%29))
  (Utilities|FlowControl|Sequence
    (:then_0
      ;[0.15 0.15 0.15 0.5] Rotate Widget
      (if (not (Variables|/Script/Engine.SceneComponent|GetbHiddenInGame (Variables|Default|GetWidget)))
        (Transformation|SetWorldRotation (Variables|Default|GetWidget) (Math|Rotator|FindLookatRotation (Transformation|GetWorldLocation (Variables|Default|GetWidget)) (Transformation|GetActorLocation (Variables|/Script/Engine.PlayerController|GetPlayerCameraManager (Game|GetPlayerController 0)))) false false)))))

(event EventUseInteractable
  (bind _playerref (Variables|Default|GetPlayerRef))
  (bind _controllerref (Variables|/Game/Variant_Combat/Blueprints/BP_CombatCharacter.BP_CombatCharacter_C|GetControllerRef _playerref))
  (Development|PrintString "Onteragit avec la note")
  (bind _returnvalue (UserInterface|CreateWidget "/Game/2_BP/UI/WBP_NoteUI.WBP_NoteUI_C" _controllerref))
  (Widget|SetVisibility (Variables|/Game/Variant_Combat/Blueprints/BP_CombatPlayerController.BP_CombatPlayerController_C|GetHUD_Ref _controllerref) "Hidden")
  (bind _output_get (Variables|/Game/Variant_Combat/Blueprints/BP_CombatPlayerController.BP_CombatPlayerController_C|SetNoteUIRef _controllerref _returnvalue))
  (UserInterface|Viewport|AddtoViewport _output_get 0))

(fn ConstructionScript
  (|CallParentFunction))