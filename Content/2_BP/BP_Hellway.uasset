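; BP_Hellway is an actor that procedurally shapes a spline into a rising spiral, with no active gameplay logic.
; The construction script loops over SpiralSegments, adding local-space points placed by cosine and sine of the index, scaled by Radius and raised by SegmentHeight per step.
; The raw index serves as the angle, and points are appended without clearing existing ones.
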(event EventBeginPlay)

(event Collision|EventActorBeginOverlap
  (params (OtherActor :type Actor%20Object%20Reference)))

(event EventTick
  (params (DeltaSeconds :type Float%20%28single-precision%29)))

(fn ConstructionScript
  (bind _radius (Variables|Default|GetRadius))
  (for _index (range 0 (Variables|Default|GetSpiralSegments))
    (Spline|AddSplinePoint (Variables|Default|GetSpline) (Math|Vector|MakeVector (* (Math|Trig|Cos(Radians) (Math|Conversions|ToFloat(Integer) _index)) _radius) (* _radius (Math|Trig|Sin(Radians) (Math|Conversions|ToFloat(Integer) _index))) (* _index (Variables|Default|GetSegmentHeight))) "Local" true)))