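; Base interactable door that the player character opens when inside its trigger box.
; Overlapping the trigger registers the door as the BP_CombatCharacter's interactable and shows a prompt widget that turns to face the camera each tick; leaving clears both.
; UseInteractable hides the prompt and plays a timeline that swings the PointDoor pivot's yaw, with door collision and re-triggering disabled until it finishes.
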(event OnComponentBeginOverlap(TriggerBox)
  (params (OverlappedComponent :type Primitive%20Component%20Object%20Reference) (OtherActor :type Actor%20Object%20Reference) (OtherComp :type Primitive%20Component%20Object%20Reference) (OtherBodyIndex :type Integer) (bFromSweep :type Boolean) (SweepResult :type Hit%20Result%20Structure%20%28by%20ref%29))
  ;[0.15 0.15 0.15 0.5] Interagir avec le character
  (bind _asbp_combat_character (Utilities|Casting|CastToBP_CombatCharacter OtherActor))
  (Variables|Default|SetPlayerRef _asbp_combat_character)
  (Default|SetInteractable (Variables|Default|GetPlayerRef) self)
  (Development|SetHiddeninGame (Variables|Default|GetWidget) false false))

(event OnComponentEndOverlap(TriggerBox)
  (params (OverlappedComponent :type Primitive%20Component%20Object%20Reference) (OtherActor :type Actor%20Object%20Reference) (OtherComp :type Primitive%20Component%20Object%20Reference) (OtherBodyIndex :type Integer))
  (bind _playerref (Variables|Default|GetPlayerRef))
  ;[0.15 0.15 0.15 0.5] Interagir avec le character
  (if (== OtherActor _playerref)
    (Default|SetInteractable _playerref)
    (Development|SetHiddeninGame (Variables|Default|GetWidget) true false)))

(event Custom|OpenDoor
  (if (not (Variables|Default|GetIsInteracting))
    (Development|SetHiddeninGame (Variables|Default|GetWidget) true false)
    (bind _angleouverture (Timeline|OuverturePorte PlayFromStart)
      (:Update
        (Variables|Default|SetIsInteracting true)
        (Transformation|SetRelativeRotation (Variables|Default|GetPointDoor) (Math|Rotator|MakeRotator 0.0 0.0 _angleouverture) false false)
        (Collision|SetCollisionEnabled (Variables|Default|GetDoor) "NoCollision"))
      (:Finished
        (Variables|Default|SetIsInteracting false)
        (Collision|SetCollisionEnabled (Variables|Default|GetDoor) "QueryAndPhysics")))))

(event EventBeginPlay
  (Development|SetHiddeninGame (Variables|Default|GetWidget) true false))

(event EventTick
  (params (DeltaSeconds :type Float%20%28single-precision%29))
  (Utilities|FlowControl|Sequence
    (:then_0
      ;[0.15 0.15 0.15 0.5] Rotate Widget
      (if (not (Variables|/Script/Engine.SceneComponent|GetbHiddenInGame (Variables|Default|GetWidget)))
        (Transformation|SetWorldRotation (Variables|Default|GetWidget) (Math|Rotator|FindLookatRotation (Transformation|GetWorldLocation (Variables|Default|GetWidget)) (Transformation|GetActorLocation (Variables|/Script/Engine.PlayerController|GetPlayerCameraManager (Game|GetPlayerController 0)))) false false)))))

(event EventUseInteractable
  (CallFunction|OpenDoor))

(fn ConstructionScript)