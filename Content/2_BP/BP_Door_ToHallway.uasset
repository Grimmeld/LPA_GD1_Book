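; Door Blueprint that moves the player to a destination and toggles them between 2D and 3D modes, named as the way to a hallway.
; Its AfterOpening event stops the player, waits briefly, then moves them to the Scene component's location.
; Leaving 2D resets the camera and, after a short delay, sets a fixed player rotation.
; Entering 2D centers the camera, removes movement and switches camera rotation mode.
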(event EventBeginPlay
  (|CallParentFunction) ; This node is disabled and will not be called.\nDrag off pins to build functionality.
)

(event Collision|EventActorBeginOverlap
  (params (OtherActor :type Actor%20Object%20Reference)))

(event EventTick
  (params (DeltaSeconds :type Float%20%28single-precision%29))
  (|CallParentFunction DeltaSeconds) ; This node is disabled and will not be called.\nDrag off pins to build functionality.
)

(event EventAfterOpening
  (bind _playerref (Variables|Default|GetPlayerRef))
  (bind _playerref_2 (Variables|Default|GetPlayerRef))
  (Default|StopPlayer _playerref)
  (Utilities|FlowControl|Delay 0.5)
  (Default|MovePlayerto _playerref (Transformation|GetWorldLocation (Variables|Default|GetScene)))
  (if (Variables|/Game/Variant_Combat/Blueprints/BP_CombatCharacter.BP_CombatCharacter_C|Getis2D _playerref)
    (Variables|/Game/Variant_Combat/Blueprints/BP_CombatCharacter.BP_CombatCharacter_C|Setis2D (Variables|Default|GetPlayerRef) false)
    (Default|ChangeRotationCamPlayer _playerref_2 false)
    (Default|ResetCamera _playerref_2)
    (Utilities|FlowControl|Delay 0.2)
    (Transformation|SetActorRotation _playerref_2 "0.000000,100.000000,0.000000")
    (else
      (Variables|/Game/Variant_Combat/Blueprints/BP_CombatCharacter.BP_CombatCharacter_C|Setis2D _playerref true)
      (Default|ChangetoCameraCenter _playerref)
      (Default|RemoveMovement _playerref)
      (Default|ChangeRotationCamPlayer _playerref true))))

(fn ConstructionScript
  (|CallParentFunction))