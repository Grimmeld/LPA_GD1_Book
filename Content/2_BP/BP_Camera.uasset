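; BP_Camera is a camera actor that pivots in place to follow the player's BP_CombatCharacter, cached on BeginPlay.
; Each Tick it yaws toward the player with a slight fixed offset, keeping its pitch and roll.
; It also traces down from the player's mesh and copies the impact height to its own Z without checking for a hit, leaving X and Y unchanged.
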(event EventBeginPlay
  (bind _asbp_combat_character (Utilities|Casting|CastToBP_CombatCharacter (Game|Player|GetPlayerPawn 0)))
  (Variables|Default|SetPlayerRef _asbp_combat_character))

(event Collision|EventActorBeginOverlap
  (params (OtherActor :type Actor%20Object%20Reference)))

(event EventTick
  (params (DeltaSeconds :type Float%20%28single-precision%29))
  (bind _returnvalue (Transformation|GetActorRotation))
  (bind _self self)
  (bind _playerref (Variables|Default|GetPlayerRef))
  (bind _returnvalue_2 (Transformation|GetActorLocation _self))
  (bind _mesh (Variables|/Script/Engine.Character|GetMesh _playerref))
  (bind (_x _y) (Math|Vector|BreakVector _returnvalue_2))
  (bind _returnvalue_3 (Transformation|GetWorldLocation _mesh))
  ;[0.15 0.15 0.15 0.5] Tourne la camera vers le joueur
  (Transformation|SetActorRotation (Math|Rotator|MakeRotator (.roll _returnvalue) (.pitch _returnvalue) (+ (.Yaw (Math|Rotator|BreakRotator (Math|Rotator|FindLookatRotation (Transformation|GetActorLocation) (.Location (Math|Transform|BreakTransform (Transformation|GetActorTransform (Variables|Default|GetPlayerRef))))))) -5.0)))
  (bind _outhit (Collision|LineTraceForObjects _returnvalue_3 (+ _returnvalue_3 (* "0.000000,0.000000,-1.000000" 1e+03)) (Variables|Default|GetObject%20Types) false (Utilities|Array|MakeArray (Variables|Default|GetPlayerRef)) "None"))
  (Transformation|SetActorLocation _self (Math|Vector|MakeVector _x _y (.Z (Math|Vector|BreakVector (.ImpactPoint (Collision|BreakHitResult _outhit))))) false false))

(fn ConstructionScript)