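; BP_Dialogue is a trigger actor that shows a one-time dialogue panel when the player's combat character walks into it.
; BeginPlay caches the player pawn as a BP_CombatCharacter reference.
; On the first Trigger overlap by such a character, it sends the name and description from Dialogues to the HUD through the player's controller, then clears the panel after the DelayMax delay.
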(event OnComponentBeginOverlap(Trigger)
  (params (OverlappedComponent :type Primitive%20Component%20Object%20Reference) (OtherActor :type Actor%20Object%20Reference) (OtherComp :type Primitive%20Component%20Object%20Reference) (OtherBodyIndex :type Integer) (bFromSweep :type Boolean) (SweepResult :type Hit%20Result%20Structure%20%28by%20ref%29))
  (bind _playerref (Variables|Default|GetPlayerRef))
  (bind _dialogues (Variables|Default|GetDialogues))
  (bind (_namechar _descr) (Utilities|Struct|BreakfDialogues _dialogues))
  (bind _controllerref (Variables|/Game/Variant_Combat/Blueprints/BP_CombatCharacter.BP_CombatCharacter_C|GetControllerRef _playerref))
  (bind _hud_ref (Variables|/Game/Variant_Combat/Blueprints/BP_CombatPlayerController.BP_CombatPlayerController_C|GetHUD_Ref _controllerref))
  (Utilities|Casting|CastToBP_CombatCharacter OtherActor)
  (if (not (Variables|Default|GetisTriggered))
    (Variables|Default|SetisTriggered true)
    (Default|AddDialoguePanel _hud_ref _namechar _descr)
    (Utilities|FlowControl|Delay (Variables|Default|GetDelayMax))
    (Default|ClearDialoguePanel _hud_ref)))

(event EventBeginPlay
  (bind _asbp_combat_character (Utilities|Casting|CastToBP_CombatCharacter (Game|Player|GetPlayerPawn 0)))
  (Variables|Default|SetPlayerRef _asbp_combat_character))

(fn ConstructionScript)