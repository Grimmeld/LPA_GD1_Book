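; BP_Door_ToConf is a door Blueprint that transitions the player out of 2D mode once it opens.
; Its AfterOpening event stops the player, clears Is2D, updates camera rotation through ChangeRotationCamPlayer and sets a fixed control yaw.
; It then resets the camera and moves the player to the world location of its Scene component.
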(event EventBeginPlay
  (|CallParentFunction) ; This node is disabled and will not be called.\nDrag off pins to build functionality.
)

(event Collision|EventActorBeginOverlap
  (params (OtherActor :type Actor%20Object%20Reference)))

(event EventTick
  (params (DeltaSeconds :type Float%20%28single-precision%29))
  (|CallParentFunction DeltaSeconds) ; This node is disabled and will not be called.\nDrag off pins to build functionality.
)

(event EventAfterOpening
  (bind _playerref (Variables|Default|GetPlayerRef))
  (bind _playerref_2 (Variables|Default|GetPlayerRef))
  (Default|StopPlayer _playerref)
  (Variables|/Game/Variant_Combat/Blueprints/BP_CombatCharacter.BP_CombatCharacter_C|Setis2D (Variables|Default|GetPlayerRef) false)
  (Default|ChangeRotationCamPlayer _playerref_2 false)
  (Pawn|SetControlRotation (Variables|/Game/Variant_Combat/Blueprints/BP_CombatCharacter.BP_CombatCharacter_C|GetControllerRef _playerref_2) (Math|Rotator|MakeRotator 0.0 0.0 104.2))
  (Default|ResetCamera _playerref_2)
  (Default|MovePlayerto _playerref (Transformation|GetWorldLocation (Variables|Default|GetScene))))

(fn ConstructionScript
  (|CallParentFunction))