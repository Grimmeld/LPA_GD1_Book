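; Interactable actor that shows a one-time dialogue panel when the player uses it.
; Its Trigger registers it with an overlapping BP_CombatCharacter and shows a prompt widget, clearing both when that character leaves.
; While visible, the widget turns each tick to face the player camera.
; UseInteractable passes the Dialogue name and description to the player's HUD, then clears the panel after a delay.
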(event OnComponentBeginOverlap(Trigger)
  (params (OverlappedComponent :type Primitive%20Component%20Object%20Reference) (OtherActor :type Actor%20Object%20Reference) (OtherComp :type Primitive%20Component%20Object%20Reference) (OtherBodyIndex :type Integer) (bFromSweep :type Boolean) (SweepResult :type Hit%20Result%20Structure%20%28by%20ref%29))
  (bind _asbp_combat_character (Utilities|Casting|CastToBP_CombatCharacter OtherActor))
  (Variables|Default|SetPlayerRef _asbp_combat_character)
  (Default|SetInteractable (Variables|Default|GetPlayerRef) self)
  (Development|SetHiddeninGame (Variables|Default|GetWidget) false false))

(event OnComponentEndOverlap(Trigger)
  (params (OverlappedComponent :type Primitive%20Component%20Object%20Reference) (OtherActor :type Actor%20Object%20Reference) (OtherComp :type Primitive%20Component%20Object%20Reference) (OtherBodyIndex :type Integer))
  (bind _playerref (Variables|Default|GetPlayerRef))
  (if (== OtherActor _playerref)
    (Default|SetInteractable _playerref)
    (Development|SetHiddeninGame (Variables|Default|GetWidget) true false)))

(event EventBeginPlay
  (|CallParentFunction)
  (Development|SetHiddeninGame (Variables|Default|GetWidget) true false))

(event Collision|EventActorBeginOverlap
  (params (OtherActor :type Actor%20Object%20Reference)))

(event EventTick
  (params (DeltaSeconds :type Float%20%28single-precision%29))
  (Utilities|FlowControl|Sequence
    (:then_0
      ;[0.15 0.15 0.15 0.5] Rotate Widget
      (if (not (Variables|/Script/Engine.SceneComponent|GetbHiddenInGame (Variables|Default|GetWidget)))
        (Transformation|SetWorldRotation (Variables|Default|GetWidget) (Math|Rotator|FindLookatRotation (Transformation|GetWorldLocation (Variables|Default|GetWidget)) (Transformation|GetActorLocation (Variables|/Script/Engine.PlayerController|GetPlayerCameraManager (Game|GetPlayerController 0)))) false false)))))

(event EventUseInteractable
  (bind _playerref (Variables|Default|GetPlayerRef))
  (bind _dialogue (Variables|Default|GetDialogue))
  (bind (_namechar _descr) (Utilities|Struct|BreakfDialogues _dialogue))
  (bind _controllerref (Variables|/Game/Variant_Combat/Blueprints/BP_CombatCharacter.BP_CombatCharacter_C|GetControllerRef _playerref))
  (bind _hud_ref (Variables|/Game/Variant_Combat/Blueprints/BP_CombatPlayerController.BP_CombatPlayerController_C|GetHUD_Ref _controllerref))
  (if (not (Variables|Default|GetisTriggered))
    (Variables|Default|SetisTriggered true)
    (Default|AddDialoguePanel _hud_ref _namechar _descr)
    (Utilities|FlowControl|Delay (Variables|Default|GetDelay))
    (Default|ClearDialoguePanel _hud_ref)))

(fn ConstructionScript
  (|CallParentFunction))